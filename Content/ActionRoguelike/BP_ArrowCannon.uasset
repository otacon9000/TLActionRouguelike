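; BP_ArrowCannon is a turret actor that aims at the player and fires magic projectiles.
; Tick rotates the whole actor every frame to face the first player pawn using a look-at rotation.
; A looping two-second timer started on BeginPlay spawns a BP_MagicProjectile at the actor's location and current rotation, with no range or line-of-sight check.
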(event Custom|OnTimerElapsed
  (Game|SpawnActorfromClass "/Game/ActionRoguelike/BP_MagicProjectile.BP_MagicProjectile_C" (Math|Transform|MakeTransform (Transformation|GetActorLocation) (Transformation|GetActorRotation)) "Undefined" 0 0))

(event EventBeginPlay
  (Utilities|Time|SetTimerbyEvent (delegate Custom|OnTimerElapsed) 2.0 true))

(event EventTick
  (params (DeltaSeconds :type Float%20%28single-precision%29))
  (Transformation|SetActorRotation (Math|Rotator|FindLookatRotation (Transformation|GetActorLocation) (Transformation|GetActorLocation (Game|Player|GetPlayerPawn 0)))))

(fn ConstructionScript)